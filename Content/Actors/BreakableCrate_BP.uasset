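; Breakable crate actor that destroys itself when an overlapping actor passes the Is Valid Attack check.
; On BeginPlay, the IsAffectedByGravity flag sets whether the crate mesh simulates physics.
; The Is Valid Attack graph holds class comparisons against the ground pound and standard attack Blueprints, but they appear unconnected to any output.
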(event OnComponentBeginOverlap(Crate)
  (params (OverlappedComponent :type Primitive%20Component%20Object%20Reference) (OtherActor :type Actor%20Object%20Reference) (OtherComp :type Primitive%20Component%20Object%20Reference) (OtherBodyIndex :type Integer) (bFromSweep :type Boolean) (SweepResult :type Hit%20Result%20Structure%20%28by%20ref%29))
  (if (|IsValidAttack OtherActor)
    (Actor|DestroyActor)))

(event EventBeginPlay
  (Physics|SetSimulatePhysics (Variables|Default|GetCrate) (Variables|Default|GetIsAffectedByGravity?)))

(fn ConstructionScript)