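; CoinGate_BP is a door that opens once the player has collected enough coins.
; When Smol_Character_BP overlaps its Box, it compares the game instance's CoinsCollected against CoinsRequired.
; On success it hides the text, moves the Cube along Z with a timeline-driven per-update world offset, then destroys itself when the timeline finishes.
; The construction script displays the required count and applies the configurable door transform.
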(event OnComponentBeginOverlap(Box)
  (params (OverlappedComponent :type Primitive%20Component%20Object%20Reference) (OtherActor :type Actor%20Object%20Reference) (OtherComp :type Primitive%20Component%20Object%20Reference) (OtherBodyIndex :type Integer) (bFromSweep :type Boolean) (SweepResult :type Hit%20Result%20Structure%20%28by%20ref%29))
  (Utilities|Casting|CastToSmol_Character_BP OtherActor)
  (if (>= (Variables|/Game/GameInstance_BP.GameInstance_BP_C|GetCoinsCollected (.AsGame%20Instance%20BP (CallFunction|GetGameInstanceBP))) (Variables|Default|GetCoinsRequired))
    (CallFunction|OpenDoor)))

(event Custom|OpenDoor
  (Development|SetHiddeninGame (Variables|Default|GetTextRender) true false)
  (bind _zvalue (Timeline|OpenTimeline Play)
    (:Update
      (bind _result (Math|Float|NegateFloat _zvalue)
        (:%20%20
          (Transformation|AddWorldOffset (Variables|Default|GetCube) (Math|Vector|MakeVector 0.0 0.0 _result) false false))))
    (:Finished
      (Actor|DestroyActor))))

(fn ConstructionScript
  (Rendering|Components|TextRender|SetText (Variables|Default|GetTextRender) (Utilities|Text|ToText(Integer) (Variables|Default|GetCoinsRequired)))
  (Transformation|SetRelativeTransform (Variables|Default|GetCube) (Variables|Default|GetDoorRelativeTransform) false false))