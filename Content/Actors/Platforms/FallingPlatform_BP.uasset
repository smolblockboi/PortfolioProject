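; A platform that falls after Smol_Character_BP steps into its PlayerDetect volume, then resets itself.
; After a configurable delay, it enables mesh physics and turns off overlap detection, while Tick counts down a fixed respawn timer.
; On expiry, it stops physics, briefly disables collision and teleports the mesh to the location saved at BeginPlay, restoring only position, not rotation.
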(event OnComponentBeginOverlap(PlayerDetect)
  (params (OverlappedComponent :type Primitive%20Component%20Object%20Reference) (OtherActor :type Actor%20Object%20Reference) (OtherComp :type Primitive%20Component%20Object%20Reference) (OtherBodyIndex :type Integer) (bFromSweep :type Boolean) (SweepResult :type Hit%20Result%20Structure%20%28by%20ref%29))
  ;[1 1 1] Player Overlap
  (bind _assmol_character_bp (Utilities|Casting|CastToSmol_Character_BP OtherActor))
  (Utilities|IsValid _assmol_character_bp
    (:Is%20Valid
      (CallFunction|StartFalling))))

(event Custom|StopFalling
  (bind _mesh (Variables|Default|GetMesh))
  ;[1 1 1] Stop Falling
  (bind _output_get (Variables|Default|SetIsFalling false))
  (Physics|SetSimulatePhysics (Variables|Default|GetMesh) _output_get)
  (Variables|/Script/Engine.PrimitiveComponent|SetbGenerateOverlapEvents (Variables|Default|GetPlayerDetect) (not _output_get))
  (Variables|Default|SetRespawnTime 5.0)
  (Collision|SetCollisionEnabled _mesh "NoCollision")
  (Utilities|FlowControl|Delay 0.1)
  (Transformation|SetWorldLocation _mesh (Variables|Default|GetRespawnLocation) false true)
  (Collision|SetCollisionEnabled _mesh "QueryAndPhysics"))

(event Custom|StartFalling
  ;[1 1 1] Start Falling
  (Utilities|FlowControl|Delay (Variables|Default|GetFallDelayTime))
  (bind _output_get (Variables|Default|SetIsFalling true))
  (Variables|/Script/Engine.PrimitiveComponent|SetbGenerateOverlapEvents (Variables|Default|GetPlayerDetect) (not _output_get))
  (Variables|Default|SetRespawnTime 5.0)
  (Physics|SetSimulatePhysics (Variables|Default|GetMesh) _output_get))

(event EventTick
  (params (DeltaSeconds :type Float%20%28single-precision%29))
  ;[1 1 1] Tick
  (if (Variables|Default|GetIsFalling)
    (if (> (Variables|Default|GetRespawnTime) 0.0)
      (Variables|Default|SetRespawnTime (- (Variables|Default|GetRespawnTime) DeltaSeconds))
      (else
        (CallFunction|StopFalling)))))

(event EventBeginPlay
  ;[1 1 1] Begin Play
  (Variables|Default|SetRespawnLocation (Transformation|GetWorldLocation (Variables|Default|GetMesh))))

(fn ConstructionScript)