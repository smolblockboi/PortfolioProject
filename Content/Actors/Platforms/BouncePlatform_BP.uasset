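; Bounce platform actor that launches the Smol character when it overlaps the trigger.
; On overlap it plays a sound, sets the character's movement mode to Walking, then launches it along the mesh's up vector scaled by a launch power variable.
; The launch overrides vertical velocity only, so horizontal momentum carries through.
; A brief vertical stretch of the mesh, reset after a short delay, gives bounce feedback.
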(event OnComponentBeginOverlap(BounceTrigger)
  (params (OverlappedComponent :type Primitive%20Component%20Object%20Reference) (OtherActor :type Actor%20Object%20Reference) (OtherComp :type Primitive%20Component%20Object%20Reference) (OtherBodyIndex :type Integer) (bFromSweep :type Boolean) (SweepResult :type Hit%20Result%20Structure%20%28by%20ref%29))
  (bind _mesh (Variables|Default|GetMesh))
  (bind _assmol_character_bp (Utilities|Casting|CastToSmol_Character_BP OtherActor))
  (Utilities|IsValid _assmol_character_bp
    (:Is%20Valid
      (Audio|Components|Audio|Play (Variables|Default|GetAudio) 0.0)
      (Pawn|Components|CharacterMovement|SetMovementMode (Variables|/Script/Engine.Character|GetCharacterMovement _assmol_character_bp) "MOVE_Walking" 0)
      (Character|LaunchCharacter _assmol_character_bp (* (Math|Vector|GetUpVector (Transformation|GetWorldRotation (Variables|Default|GetMesh))) (* (Variables|Default|GetLauchPower) 1e+03)) false true)
      (Transformation|SetRelativeScale3D _mesh "1.000000,1.000000,1.500000")
      (Utilities|FlowControl|Delay 0.2)
      (Transformation|SetRelativeScale3D _mesh "1.000000,1.000000,1.000000"))))

(fn ConstructionScript)