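; Moving platform actor that uses InterpToMovement to travel between its origin and a configurable relative EndPosition.
; The construction script sets the movement duration, adds both control points and stretches a SplineMesh along the same path, multiplying its end point by 100.
; On BeginPlay the SplineMesh detaches with its world transform kept, so the path mesh stays in place while the platform moves.
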(event EventBeginPlay
  (Transformation|DetachFromComponent (Variables|Default|GetSplineMesh) "KeepWorld" "KeepWorld" "KeepWorld" true))

(fn ConstructionScript
  (bind _endposition (Variables|Default|GetEndPosition))
  (bind _splinemesh (Variables|Default|GetSplineMesh))
  (bind _interptomovement (Variables|Default|GetInterpToMovement))
  (Variables|/Script/Engine.InterpToMovementComponent|SetDuration (Variables|Default|GetInterpToMovement) (Variables|Default|GetMoveDuration))
  (Utilities|FlowControl|Sequence
    (:then_0
      (SplineMesh|SetStartPosition _splinemesh "0, 0, 0" true)
      (SplineMesh|SetEndPosition _splinemesh (/ _endposition 0.01) true))
    (:then_1
      (Class|InterptoMovementComponent|AddControlPointPosition _interptomovement "0, 0, 0" true)
      (Class|InterptoMovementComponent|AddControlPointPosition _interptomovement _endposition true))))