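; Coin cluster collectible that lays out a configurable arc of coin meshes in its Construction Script.
; Coins step along local X by Spacing, with height taken from a forward vector pitched across roughly 180 degrees, scaled by Apex and raised slightly.
; SkipFirst starts the loop at index 1, omitting the coin at the arc's origin.
; Each coin's world rotation and scale are reset, independent of the actor's transform.
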(fn ConstructionScript
  (if (Variables|Default|GetSkipFirst?)
    (Variables|Default|SetStartIndex 1))
  (for _index (range (Variables|Default|GetStartIndex) (+ (Variables|Default|GetCoinCount) (- (Variables|Default|GetStartIndex) 1)))
    (bind _returnvalue (AddComponent|AddCoinMeshComponent false (Math|Transform|MakeTransform (+ (Math|Vector|MakeVector (* _index (Variables|Default|GetSpacing)) (.y (* (Math|Vector|GetForwardVector (Math|Rotator|MakeRotator 0.0 (Math|Conversions|ToFloat(Integer) (* _index (/ 180 (+ (Variables|Default|GetCoinCount) (- (Variables|Default|GetStartIndex) 1))))) 0.0)) (Variables|Default|GetApex))) (.z (* (Math|Vector|GetForwardVector (Math|Rotator|MakeRotator 0.0 (Math|Conversions|ToFloat(Integer) (* _index (/ 180 (+ (Variables|Default|GetCoinCount) (- (Variables|Default|GetStartIndex) 1))))) 0.0)) (Variables|Default|GetApex)))) "0, 0,40.000000") "0, 0, 0" "1,1,1")))
    (Transformation|SetWorldRotation _returnvalue "0, 0, 0" false false)
    (Transformation|SetWorldScale3D _returnvalue "1.000000,1.000000,1.000000")))