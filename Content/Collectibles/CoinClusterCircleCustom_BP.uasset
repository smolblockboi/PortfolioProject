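; Collectible coin cluster that lays out a configurable number of coin meshes in a horizontal ring.
; The construction script adds each mesh at a yaw-stepped forward vector scaled by CircleRadius, raised slightly above the origin.
; Each coin's world rotation and scale are reset, so all share one orientation and size.
; The angle step uses integer division, so spacing is uneven when CoinCount does not divide 360.
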(fn ConstructionScript
  (bind _coincount (Variables|Default|GetCoinCount))
  (for _index (range 1 _coincount)
    (bind _returnvalue (AddComponent|AddCoinMeshComponent false (Math|Transform|MakeTransform (+ (* (Math|Vector|GetForwardVector (Math|Rotator|MakeRotator 0.0 0.0 (Math|Conversions|ToFloat(Integer) (* _index (/ 360 _coincount))))) (Variables|Default|GetCircleRadius)) "0, 0,40.000000") "0, 0, 0" "1,1,1")))
    (Transformation|SetWorldRotation _returnvalue "0, 0, 0" false false)
    (Transformation|SetWorldScale3D _returnvalue "1.000000,1.000000,1.000000")))