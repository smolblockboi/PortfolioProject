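; Collectible ability pickup with a spinning mesh and text label that unlocks its listed abilities when the player character touches it.
; Construction fills the label from the first ability's class name if no text is set, or a default if none is valid.
; On overlap it unlocks through the GameInstance, hides, triggers the character's get-item animation and shows an ItemGot widget.
; The animation-finished callback removes the widget and destroys the pickup.
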(event OnComponentBeginOverlap(Sphere)
  (params (OverlappedComponent :type Primitive%20Component%20Object%20Reference) (OtherActor :type Actor%20Object%20Reference) (OtherComp :type Primitive%20Component%20Object%20Reference) (OtherBodyIndex :type Integer) (bFromSweep :type Boolean) (SweepResult :type Hit%20Result%20Structure%20%28by%20ref%29))
  (bind _assmol_character_bp (Utilities|Casting|CastToSmol_Character_BP OtherActor))
  (EventDispatchers|BindEventtoGetItemAnimationFinished _assmol_character_bp (delegate Custom|DestroyWidget))
  (for _array_element (Variables|Default|GetAbilitiesGained)
    (Default|UnlockAbility (.AsGame%20Instance%20BP (CallFunction|GetGameInstanceBP)) _array_element))
  (Rendering|SetActorHiddenInGame true)
  (Default|GotItem _assmol_character_bp)
  (CallFunction|MakeNewWidget)
  (Variables|/Script/Engine.PrimitiveComponent|SetbGenerateOverlapEvents (Variables|Default|GetSphere) false))

(event Custom|MakeNewWidget
  (bind _returnvalue (UserInterface|CreateWidget "/Game/Collectibles/ItemGot_Widget.ItemGot_Widget_C" (Game|GetPlayerController 0)))
  (bind _output_get (Variables|Default|SetItemGotWidget _returnvalue))
  (Variables|/Game/Collectibles/ItemGot_Widget.ItemGot_Widget_C|SetItemString _output_get (Utilities|String|ToString(Text) (Variables|Default|GetAbilityText)))
  (UserInterface|Viewport|AddtoPlayerScreen _output_get))

(event Custom|DestroyWidget
  (Widget|RemovefromParent (Variables|Default|GetItemGotWidget))
  (Actor|DestroyActor))

(event EventTick
  (params (DeltaSeconds :type Float%20%28single-precision%29))
  (Transformation|AddLocalRotation (Variables|Default|GetMesh) (* (Math|Rotator|MakeRotator 0.0 0.0 1.8e+02) DeltaSeconds) false false))

(fn ConstructionScript
  (bind _textrender (Variables|Default|GetTextRender))
  (bind _abilitiesgained (Variables|Default|GetAbilitiesGained))
  (bind _output (Utilities|Array|Get(acopy) _abilitiesgained))
  (if (Utilities|IsValidClass _output)
    (if (Utilities|Enum|Equal(Enum) (Variables|Default|GetAbilityText) (Utilities|Text|MakeLiteralText ""))
      (Variables|Default|SetAbilityText (Utilities|Text|ToText(String) (Utilities|GetClassDisplayName _output))))
    (Rendering|Components|TextRender|SetText _textrender (Variables|Default|GetAbilityText))
    (else
      (bind _output_get (Variables|Default|SetAbilityText (LocalVariables|GetDefaultText)))
      (Rendering|Components|TextRender|SetText _textrender _output_get))))