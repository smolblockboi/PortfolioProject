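; Collectible coin cluster Blueprint that lays out a configurable line of coin meshes when constructed.
; The construction script adds one mesh component per coin along the actor's local X axis at a set spacing, raised by an offset from the actor's up vector.
; SkipFirst shifts the line one slot forward while keeping the coin count.
; Each coin's world rotation and scale are then reset, so coins ignore the actor's rotation and scale.
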(fn ConstructionScript
  (if (Variables|Default|GetSkipFirst?)
    (Variables|Default|SetStartIndex 1))
  (for _index (range (Variables|Default|GetStartIndex) (+ (Variables|Default|GetCoin%20Count) (- (Variables|Default|GetStartIndex) 1)))
    (bind _returnvalue (AddComponent|AddCoinMeshComponent false (Math|Transform|MakeTransform (+ (* (Math|Vector|GetForwardVector "0, 0, 0") (* _index (Variables|Default|GetSpacing))) (* (Math|Vector|GetUpVector (Transformation|GetActorRotation)) 4e+01)) "0, 0, 0" "1.000000,10.000000,1.000000")))
    (Transformation|SetWorldRotation _returnvalue "0, 0, 0" false false)
    (Transformation|SetWorldScale3D _returnvalue "1.000000,1.000000,1.000000")))