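; LevelTransition_BP is a trigger that moves the player to another level.
; When a Smol_Character_BP overlaps its Cube, it calls OpenTargetLevel with a level reference and a debug level name.
; Its construction script labels the TextRender with the destination, showing the reference in packaged-for-distribution builds and the debug name otherwise.
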(event OnComponentBeginOverlap(Cube)
  (params (OverlappedComponent :type Primitive%20Component%20Object%20Reference) (OtherActor :type Actor%20Object%20Reference) (OtherComp :type Primitive%20Component%20Object%20Reference) (OtherBodyIndex :type Integer) (bFromSweep :type Boolean) (SweepResult :type Hit%20Result%20Structure%20%28by%20ref%29))
  (Utilities|Casting|CastToSmol_Character_BP OtherActor)
  (CallFunction|OpenTargetLevel (Variables|Default|GetTargetLevelReference) (Variables|Default|GetDebugTargetLevelName)))

(fn ConstructionScript
  (bind _textrender (Variables|Default|GetTextRender))
  (if (Class|KismetSystemLibrary|IsPackagedforDistribution)
    (Rendering|Components|TextRender|SetText _textrender (Utilities|Text|ToText(String) (Utilities|String|Append "To: 
" (Utilities|ToString(SoftObjectReference) (Variables|Default|GetTargetLevelReference)))))
    (else
      (Rendering|Components|TextRender|SetText _textrender (Utilities|Text|ToText(String) (Utilities|String|Append "To: " (Utilities|String|ToString(Name) (Variables|Default|GetDebugTargetLevelName))))))))