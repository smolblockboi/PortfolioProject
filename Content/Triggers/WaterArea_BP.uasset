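; WaterArea_BP is a trigger area that lets Smol_Character_BP swim while overlapping it.
; On begin overlap it flags the character's current physics volume as water and sets movement to Swimming; on end overlap it clears the flag and sets Falling.
; The flag is written on whatever volume GetPhysicsVolume returns.
; The construction script sizes the Cube component from AreaScale with a fixed multiplier.
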(event Collision|EventActorBeginOverlap
  (params (OtherActor :type Actor%20Object%20Reference))
  (bind _assmol_character_bp (Utilities|Casting|CastToSmol_Character_BP OtherActor))
  (Variables|/Script/Engine.PhysicsVolume|SetbWaterVolume (Class|MovementComponent|GetPhysicsVolume (Variables|/Script/Engine.Character|GetCharacterMovement _assmol_character_bp)) true)
  (Pawn|Components|CharacterMovement|SetMovementMode (Variables|/Script/Engine.Character|GetCharacterMovement _assmol_character_bp) "MOVE_Swimming" 0))

(event Collision|EventActorEndOverlap
  (params (OtherActor :type Actor%20Object%20Reference))
  (bind _assmol_character_bp (Utilities|Casting|CastToSmol_Character_BP OtherActor))
  (Variables|/Script/Engine.PhysicsVolume|SetbWaterVolume (Class|MovementComponent|GetPhysicsVolume (Variables|/Script/Engine.Character|GetCharacterMovement _assmol_character_bp)) false)
  (Pawn|Components|CharacterMovement|SetMovementMode (Variables|/Script/Engine.Character|GetCharacterMovement _assmol_character_bp) "MOVE_Falling" 0))

(fn ConstructionScript
  (Transformation|SetRelativeScale3D (Variables|Default|GetCube) (* (Variables|Default|GetAreaScale) 0.65)))