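; Swim component for the Smol character that gives it an upward swim stroke.
; On BeginPlay it casts its owner to Smol_Character_BP and binds DoSwim to that character's attempt-swim event.
; Each stroke zeroes vertical velocity, then adds a fixed velocity-change impulse along the actor's up vector, so every stroke gives the same lift regardless of falling speed.
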(event Custom|DoSwim
  (bind _as_smol_character_bp (Variables|Default|GetAs%20Smol%20Character%20BP))
  (bind _charactermovement (Variables|/Script/Engine.Character|GetCharacterMovement _as_smol_character_bp))
  (Variables|/Script/Engine.MovementComponent|SetVelocity _charactermovement (Math|Vector|MakeVector (.x (Variables|/Script/Engine.MovementComponent|GetVelocity _charactermovement)) (.y (Variables|/Script/Engine.MovementComponent|GetVelocity _charactermovement)) 0.0))
  (Physics|AddImpulse _charactermovement (* (Math|Vector|GetUpVector (Transformation|GetActorRotation _as_smol_character_bp)) 7.5e+02) true))

(event EventBeginPlay
  (bind _assmol_character_bp (Utilities|Casting|CastToSmol_Character_BP (Components|GetOwner)))
  (bind _output_get (Variables|Default|SetAs%20Smol%20Character%20BP _assmol_character_bp))
  (EventDispatchers|BindEventtoAttemptSwim _output_get (delegate Custom|DoSwim)))