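; Ground pound attack actor that watches the player's Smol character and signals how the attack ends.
; It caches player 0's pawn on BeginPlay and checks its movement state every tick while airborne.
; Landing on the ground fires EndedOnGround, while climbing or swimming fires EndedEarly.
; Either outcome destroys the actor, and the pound's motion and damage are not handled in this graph.
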(event EventBeginPlay
  (bind _assmol_character_bp (Utilities|Casting|CastToSmol_Character_BP (Game|Player|GetPlayerPawn 0)))
  (Variables|Default|SetAs%20Smol%20Character%20BP _assmol_character_bp))

(event EventTick
  (params (DeltaSeconds :type Float%20%28single-precision%29))
  (bind _as_smol_character_bp (Variables|Default|GetAs%20Smol%20Character%20BP))
  (bind _charactermovement (Variables|/Script/Engine.Character|GetCharacterMovement _as_smol_character_bp))
  (bind _isclimbing_ (Variables|/Game/Smol/Smol_Character_BP.Smol_Character_BP_C|GetIsClimbing? _as_smol_character_bp))
  (bind _returnvalue (AI|Components|NavMovement|IsFalling _charactermovement))
  (bind _returnvalue_2 (AI|Components|NavMovement|IsSwimming _charactermovement :!class /Script/Engine.NavMovementComponent))
  (bind _returnvalue_3 (not _returnvalue))
  (Utilities|IsValid (Variables|Default|GetAs%20Smol%20Character%20BP)
    (:Is%20Valid
      (if (Math|Boolean|ORBoolean _isclimbing_ _returnvalue_3 _returnvalue_2) ; Is Climbing OR Not Falling OR Swimming?
        (if (Math|Boolean|ANDBoolean (not _isclimbing_) _returnvalue_3 (not _returnvalue_2)) ; Is Not Climbing AND Not Falling AND Not Swimming?
          (Default|CallEndedonGround)
          (Actor|DestroyActor :!label _label)
          (elif (or _isclimbing_ _returnvalue_2)
            (Default|CallEndedEarly)
            (goto _label)))))))

(fn ConstructionScript)