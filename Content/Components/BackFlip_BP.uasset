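; Actor component that gives Smol_Character_BP a backflip move.
; On BeginPlay it casts its owner and binds DoBackflip to the character's AttemptBackflip event.
; The flip flags the character, uncrouches, jumps with doubled JumpZVelocity and adds a backward velocity-change impulse scaled from that jump speed, storing the direction.
; After a short delay it clears the flag and restores base jump velocity.
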(event Custom|DoBackflip
  (CallFunction|BackflipStart)
  (Utilities|FlowControl|Delay 0.2)
  (CallFunction|BackflipEnd))

(event EventBeginPlay
  (bind _assmol_character_bp (Utilities|Casting|CastToSmol_Character_BP (Components|GetOwner)))
  (bind _output_get (Variables|Default|SetAs%20Smol%20Character%20BP _assmol_character_bp))
  (EventDispatchers|BindEventtoAttemptBackflip _output_get (delegate Custom|DoBackflip)))

(fn BackflipStart
  (bind _as_smol_character_bp (Variables|Default|GetAs%20Smol%20Character%20BP))
  (bind _returnvalue (Transformation|GetActorForwardVector _as_smol_character_bp))
  (bind _charactermovement (Variables|/Script/Engine.Character|GetCharacterMovement _as_smol_character_bp))
  (bind _basejumpzvelocity (Variables|/Game/Smol/Smol_Character_BP.Smol_Character_BP_C|GetBaseJumpZVelocity _as_smol_character_bp))
  (bind _returnvalue_2 (Math|Vector|NegateVector _returnvalue))
  (bind _returnvalue_3 (* _basejumpzvelocity 2.0))
  (Variables|/Game/Smol/Smol_Character_BP.Smol_Character_BP_C|SetIsBackflipping? _as_smol_character_bp true)
  (Character|UnCrouch _as_smol_character_bp)
  (Variables|/Script/Engine.CharacterMovementComponent|SetJumpZVelocity _charactermovement _returnvalue_3)
  (Character|Jump _as_smol_character_bp)
  (Physics|AddImpulse _charactermovement (* _returnvalue_2 (* _returnvalue_3 0.7)) true)
  (Variables|Default|SetBackflipDirection _returnvalue_2))

(fn BackflipEnd
  (bind _as_smol_character_bp (Variables|Default|GetAs%20Smol%20Character%20BP))
  (Variables|/Game/Smol/Smol_Character_BP.Smol_Character_BP_C|SetIsBackflipping? _as_smol_character_bp false)
  (Variables|/Script/Engine.CharacterMovementComponent|SetJumpZVelocity (Variables|/Script/Engine.Character|GetCharacterMovement _as_smol_character_bp) (Variables|/Game/Smol/Smol_Character_BP.Smol_Character_BP_C|GetBaseJumpZVelocity _as_smol_character_bp)))