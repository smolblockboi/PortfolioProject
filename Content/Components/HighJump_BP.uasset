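; HighJump_BP is a component that gives the owning Smol_Character_BP a high jump.
; On BeginPlay it binds to the character's AttemptHighJump event.
; When fired, it uncrouches, sets the spin-jumping flag, doubles jump Z velocity from its base value and jumps.
; After a short delay it clears the flag and restores the base jump velocity.
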(event Custom|DoHighJump
  (CallFunction|HighJumpStart)
  (Utilities|FlowControl|Delay 0.2)
  (CallFunction|HighJumpEnd))

(event EventBeginPlay
  (bind _assmol_character_bp (Utilities|Casting|CastToSmol_Character_BP (Components|GetOwner)))
  (bind _output_get (Variables|Default|SetAs%20Smol%20Character%20BP _assmol_character_bp))
  (EventDispatchers|BindEventtoAttemptHighJump _output_get (delegate Custom|DoHighJump)))

(fn HighJumpStart
  (bind _as_smol_character_bp (Variables|Default|GetAs%20Smol%20Character%20BP))
  (Variables|/Game/Smol/Smol_Character_BP.Smol_Character_BP_C|SetIsSpinJumping? _as_smol_character_bp true)
  (Character|UnCrouch _as_smol_character_bp)
  (Variables|/Script/Engine.CharacterMovementComponent|SetJumpZVelocity (Variables|/Script/Engine.Character|GetCharacterMovement _as_smol_character_bp) (* (Variables|/Game/Smol/Smol_Character_BP.Smol_Character_BP_C|GetBaseJumpZVelocity _as_smol_character_bp) 2.0))
  (Character|Jump _as_smol_character_bp))

(fn HighJumpEnd
  (bind _as_smol_character_bp (Variables|Default|GetAs%20Smol%20Character%20BP))
  (Variables|/Game/Smol/Smol_Character_BP.Smol_Character_BP_C|SetIsSpinJumping? _as_smol_character_bp false)
  (Variables|/Script/Engine.CharacterMovementComponent|SetJumpZVelocity (Variables|/Script/Engine.Character|GetCharacterMovement _as_smol_character_bp) (Variables|/Game/Smol/Smol_Character_BP.Smol_Character_BP_C|GetBaseJumpZVelocity _as_smol_character_bp)))