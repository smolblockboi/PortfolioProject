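; Wall-climb component for Smol_Character_BP that grabs walls when the character falls while pushing toward one.
; Climbing uses Flying movement, attaches the character to the wall component and uses sphere traces each Tick to align it to the surface.
; Floor contact, physics-simulating surfaces or jump attempts end the climb.
; Losing the wall with forward input triggers a ledge hop with a delayed forward impulse and briefly disabled input.
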(event Custom|StartClimb
  (bind _as_smol_character_bp (Variables|Default|GetAs%20Smol%20Character%20BP))
  (bind _charactermovement (Variables|/Script/Engine.Character|GetCharacterMovement _as_smol_character_bp))
  ;[1 1 1] Start Climbing
  (bind (_outhit _hashit_) (CallFunction|GetWallClimbTrace))
  (if _hashit_
    (Variables|/Game/Smol/Smol_Character_BP.Smol_Character_BP_C|SetIsClimbing? _as_smol_character_bp true)
    (Pawn|Components|CharacterMovement|SetMovementMode _charactermovement "MOVE_Flying" 0)
    (Components|Movement|StopMovementImmediately _charactermovement)
    (Variables|/Script/Engine.CharacterMovementComponent|SetbOrientRotationToMovement _charactermovement false)
    (CallFunction|SetWallClimbLocationandRotation _as_smol_character_bp (.Location (Collision|BreakHitResult _outhit)) (.Normal (Collision|BreakHitResult _outhit)))
    (CallFunction|AttachPlayertoComponent (.HitComponent (Collision|BreakHitResult _outhit)))))

(event Custom|StopClimbing
  (bind _as_smol_character_bp (Variables|Default|GetAs%20Smol%20Character%20BP))
  (bind _charactermovement (Variables|/Script/Engine.Character|GetCharacterMovement _as_smol_character_bp))
  ;[1 1 1] Stop Climbing
  (Variables|/Game/Smol/Smol_Character_BP.Smol_Character_BP_C|SetIsClimbing? _as_smol_character_bp false)
  (Variables|/Script/Engine.CharacterMovementComponent|SetbOrientRotationToMovement _charactermovement true)
  (Pawn|Components|CharacterMovement|SetMovementMode _charactermovement "MOVE_Falling" 0)
  (CallFunction|DetachPlayer))

(event Custom|LedgeHop
  (bind _as_smol_character_bp (Variables|Default|GetAs%20Smol%20Character%20BP))
  (bind _charactermovement (Variables|/Script/Engine.Character|GetCharacterMovement _as_smol_character_bp))
  ;[1 1 1] Ledge Hop
  (Utilities|FlowControl|Sequence
    (:then_0
      (Variables|/Game/Smol/Smol_Character_BP.Smol_Character_BP_C|SetIsClimbing? _as_smol_character_bp false)
      (Variables|/Script/Engine.CharacterMovementComponent|SetbOrientRotationToMovement _charactermovement true)
      (Pawn|Components|CharacterMovement|SetMovementMode _charactermovement "MOVE_Falling" 0))
    (:then_1
      (Input|DisableInput _as_smol_character_bp 0)
      (Character|Jump _as_smol_character_bp)
      (bind _returnvalue (CallFunction|GetLedgeHopDirection))
      (Utilities|FlowControl|Delay 0.1)
      (Physics|AddImpulse _charactermovement (* _returnvalue 2e+02) true)
      (Utilities|FlowControl|Delay 0.5)
      (Input|EnableInput _as_smol_character_bp 0)
      (CallFunction|DetachPlayerfromComponent))))

(event EventBeginPlay
  (bind _assmol_character_bp (Utilities|Casting|CastToSmol_Character_BP (Components|GetOwner)))
  (bind _output_get (Variables|Default|SetAs%20Smol%20Character%20BP _assmol_character_bp))
  (EventDispatchers|BindEventtoAttemptJumpWhileClimbing _output_get (delegate Custom|StopClimbing)))

(event EventTick
  (params (DeltaSeconds :type Float%20%28single-precision%29))
  (bind _as_smol_character_bp (Variables|Default|GetAs%20Smol%20Character%20BP))
  (bind _charactermovement (Variables|/Script/Engine.Character|GetCharacterMovement _as_smol_character_bp))
  (bind _isclimbing_ (Variables|/Game/Smol/Smol_Character_BP.Smol_Character_BP_C|GetIsClimbing? _as_smol_character_bp))
  ;[1 1 1] Climbing Tick
  (if _isclimbing_
    (bind _returnvalue (CallFunction|GetFloorTrace))
    (if (and (not _returnvalue) _isclimbing_)
      (bind (_outhit _hashit_) (CallFunction|GetWallClimbTrace))
      (if _hashit_
        (if (not (Physics|IsSimulatingPhysics (.HitComponent (Collision|BreakHitResult _outhit)) "None"))
          (CallFunction|SetWallClimbLocationandRotation (Variables|Default|GetAs%20Smol%20Character%20BP) (.Location (Collision|BreakHitResult _outhit)) (.Normal (Collision|BreakHitResult _outhit)))
          (else
            (CallFunction|StopClimbing :!label _label)))
        (elif (> (Variables|/Game/Smol/Smol_Character_BP.Smol_Character_BP_C|GetInputAxisForward (Variables|Default|GetAs%20Smol%20Character%20BP)) 0.0)
          (CallFunction|LedgeHop)
          (else
            (goto _label))))
      (else
        (goto _label)))
    (elif (Math|Boolean|ANDBoolean (|IsInputTowardWall? _as_smol_character_bp) (AI|Components|NavMovement|IsFalling _charactermovement) (< (.z (Pawn|Components|CharacterMovement|GetLastUpdateVelocity _charactermovement)) 0.0))
      (bind (_outhit_2 _hashit__2) (CallFunction|GetWallClimbTrace))
      (if _hashit__2
        (if (not (Physics|IsSimulatingPhysics (.HitComponent (Collision|BreakHitResult _outhit_2)) "None"))
          (CallFunction|StartClimb))))))

(fn GetWallClimbTrace
  (bind _walltraceforwardoffset (Variables|Default|GetWallTraceForwardOffset))
  (bind _as_smol_character_bp (Variables|Default|GetAs%20Smol%20Character%20BP))
  (bind _returnvalue (Transformation|GetActorForwardVector _as_smol_character_bp))
  (bind _returnvalue_2 (Transformation|GetActorLocation _as_smol_character_bp))
  (bind _returnvalue_3 (* _returnvalue _walltraceforwardoffset))
  (bind _returnvalue_4 (+ _returnvalue_2 _returnvalue_3))
  (bind (_outhit _returnvalue_5) (Collision|SphereTraceByChannel _returnvalue_4 (+ _returnvalue_4 (* (Math|Vector|GetForwardVector (Transformation|GetActorRotation _as_smol_character_bp)) (Variables|Default|GetWallDistance))) (Variables|Default|GetWallSphereTraceRadius) "TraceTypeQuery1" false 0 (Variables|Default|GetDraw%20Debug%20Type)))
  (if _returnvalue_5
    (Variables|/Game/Smol/Smol_Character_BP.Smol_Character_BP_C|SetClimb%20Right%20Vector (Variables|Default|GetAs%20Smol%20Character%20BP) (* (Math|Vector|GetRightVector (Math|Rotator|MakeRotfromX (.Normal (Collision|BreakHitResult _outhit)))) -1.0)))
  (return _outhit _returnvalue_5))

(fn SetWallClimbLocationandRotation
  (params (SmolCharacterRef :type Smol%20Character%20BP%20Object%20Reference) (HitLocation :type Vector) (HitNormal :type Vector%20%28by%20ref%29))
  (bind _returnvalue (Transformation|GetActorRotation SmolCharacterRef))
  (bind _returnvalue_2 (Transformation|GetActorForwardVector SmolCharacterRef))
  (bind _walltraceforwardoffset (Variables|Default|GetWallTraceForwardOffset))
  (bind _returnvalue_3 (* _returnvalue_2 _walltraceforwardoffset))
  (bind _returnvalue_4 (- HitLocation _returnvalue_3))
  (Transformation|SetActorLocationAndRotation SmolCharacterRef (Math|Vector|MakeVector (.x _returnvalue_4) (.y _returnvalue_4) (.z (Transformation|GetActorLocation SmolCharacterRef))) (Math|Rotator|MakeRotator (.roll _returnvalue) (.pitch _returnvalue) (+ (.yaw (Math|Rotator|MakeRotfromX HitNormal)) 1.8e+02)) true))

(fn GetFloorTrace
  (bind _as_smol_character_bp (Variables|Default|GetAs%20Smol%20Character%20BP))
  (bind _returnvalue (Transformation|GetActorLocation _as_smol_character_bp))
  (bind (_outhit _returnvalue_2) (Collision|SphereTraceByChannel _returnvalue (+ _returnvalue (* (Math|Vector|NegateVector (Math|Vector|GetUpVector (Transformation|GetActorRotation _as_smol_character_bp))) (Variables|Default|GetFloorDistance))) (Variables|Default|GetFloorSphereTraceRadius) "TraceTypeQuery1" false 0 (Variables|Default|GetDraw%20Debug%20Type)))
  (return _outhit _returnvalue_2))

(fn GetLedgeHopDirection
  (return (Math|Vector|GetForwardVector (Transformation|GetActorRotation (Variables|Default|GetAs%20Smol%20Character%20BP)))))

(fn AttachPlayer
  (params (PrimitiveComponent :type Primitive%20Component%20Object%20Reference))
  (Transformation|AttachComponentToComponent (Variables|Default|GetAs%20Smol%20Character%20BP) PrimitiveComponent "None" "KeepWorld" "KeepWorld" "KeepWorld" true))

(fn DetachPlayer
  (Transformation|DetachFromActor (Variables|Default|GetAs%20Smol%20Character%20BP) "KeepWorld" "KeepWorld" "KeepWorld"))