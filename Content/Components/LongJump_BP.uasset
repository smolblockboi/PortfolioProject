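; LongJump_BP is an actor component that gives Smol_Character_BP a long jump out of a crouch.
; On BeginPlay it casts its owner and binds to the character's crouch-start and long-jump-attempt events.
; Starting a crouch opens a brief timed window through the character's CanLongJump flag.
; An attempt inside that window while still crouching launches the character forward and upward, overriding its current velocity.
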(event Custom|DoLongJump
  (bind _as_smol_character_bp (Variables|Default|GetAs%20Smol%20Character%20BP))
  (bind _returnvalue (Transformation|GetActorForwardVector _as_smol_character_bp))
  (if (and (Variables|/Game/Smol/Smol_Character_BP.Smol_Character_BP_C|GetCanLongJump? _as_smol_character_bp) (AI|Components|NavMovement|IsCrouching (Variables|/Script/Engine.Character|GetCharacterMovement _as_smol_character_bp)))
    (Character|LaunchCharacter _as_smol_character_bp (Math|Vector|MakeVector (* (.x _returnvalue) 1e+03) (* (.y _returnvalue) 1e+03) (+ (.z _returnvalue) 8e+02)) true true)))

(event Custom|CrouchStarted
  (bind _as_smol_character_bp (Variables|Default|GetAs%20Smol%20Character%20BP))
  (Variables|/Game/Smol/Smol_Character_BP.Smol_Character_BP_C|SetCanLongJump? _as_smol_character_bp true)
  (Utilities|FlowControl|Delay 0.2)
  (Variables|/Game/Smol/Smol_Character_BP.Smol_Character_BP_C|SetCanLongJump? _as_smol_character_bp false))

(event EventBeginPlay
  (bind _assmol_character_bp (Utilities|Casting|CastToSmol_Character_BP (Components|GetOwner)))
  (bind _output_get (Variables|Default|SetAs%20Smol%20Character%20BP _assmol_character_bp))
  (EventDispatchers|BindEventtoStartedCrouching _output_get (delegate Custom|CrouchStarted))
  (EventDispatchers|BindEventtoAttemptLongJump _output_get (delegate Custom|DoLongJump)))

(fn StartLongJump)