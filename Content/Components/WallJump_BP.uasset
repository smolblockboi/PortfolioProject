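; Actor component that gives Smol_Character_BP two wall moves, a jump away and a vertical hop.
; On BeginPlay it binds to the character's wall jump attempt event and picks a move by whether movement input points behind the player.
; The jump launches backward and up, then turns the character around, while the hop launches only upward.
; Both scale launch speed from the character's base jump velocity.
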(event Custom|DoWallHop
  (bind _as_smol_character_bp (Variables|Default|GetAs%20Smol%20Character%20BP))
  (Character|LaunchCharacter _as_smol_character_bp (Math|Vector|MakeVector 0.0 0.0 (* (Variables|/Game/Smol/Smol_Character_BP.Smol_Character_BP_C|GetBaseJumpZVelocity _as_smol_character_bp) 1.5)) false true))

(event Custom|DoWallJump
  (bind _as_smol_character_bp (Variables|Default|GetAs%20Smol%20Character%20BP))
  (bind _basejumpzvelocity (Variables|/Game/Smol/Smol_Character_BP.Smol_Character_BP_C|GetBaseJumpZVelocity _as_smol_character_bp))
  (bind _returnvalue (* _basejumpzvelocity 1.5))
  (bind _mirroredvector (CallFunction|FlipCharacterAround))
  (Character|LaunchCharacter _as_smol_character_bp (+ (* _mirroredvector _returnvalue) (Math|Vector|MakeVector 0.0 0.0 _returnvalue)) true true)
  (Transformation|SetActorRotation _as_smol_character_bp (Math|Rotator|MakeRotator 0.0 0.0 (- (.yaw (Transformation|GetActorRotation _as_smol_character_bp)) 1.8e+02)) true))

(event Custom|HandleWallJumpType
  (bind _as_smol_character_bp (Variables|Default|GetAs%20Smol%20Character%20BP))
  (if (CallFunction|IsInputBehindPlayer? (Variables|/Game/Smol/Smol_Character_BP.Smol_Character_BP_C|GetInputAxisForward _as_smol_character_bp) (Variables|/Game/Smol/Smol_Character_BP.Smol_Character_BP_C|GetInputAxisRight _as_smol_character_bp))
    (CallFunction|DoWallJump)
    (else
      (CallFunction|DoWallHop))))

(event EventBeginPlay
  (bind _assmol_character_bp (Utilities|Casting|CastToSmol_Character_BP (Components|GetOwner)))
  (bind _output_get (Variables|Default|SetAs%20Smol%20Character%20BP _assmol_character_bp))
  (EventDispatchers|BindEventtoAttemptWallJump _output_get (delegate Custom|HandleWallJumpType)))

(fn FlipCharacterAround
  (return (Math|Vector|NegateVector (Math|Vector|GetForwardVector (Math|Rotator|MakeRotator 0.0 0.0 (.yaw (Transformation|GetActorRotation (Variables|Default|GetAs%20Smol%20Character%20BP))))))))