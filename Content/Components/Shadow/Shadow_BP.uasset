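; Actor component that gives its owner a mesh-based drop shadow on the surface beneath it.
; On BeginPlay it adds a shadow mesh component to the owner at a configurable scale.
; Each tick it line-traces along the owner's down vector and moves the mesh to just below the hit point.
; Roll and pitch follow the surface normal while yaw follows the owner, with no check for a missed trace.
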(event EventBeginPlay
  (bind _returnvalue (Game|AddComponentbyClass (Components|GetOwner) "/Game/Components/Shadow/Shadow_Mesh_Component.Shadow_Mesh_Component_C" false (Math|Transform|MakeTransform "0, 0, 0" "0, 0, 0" (Variables|Default|GetShadowScale))))
  (Variables|Default|SetShadowComponent _returnvalue))

(event EventTick
  (params (DeltaSeconds :type Float%20%28single-precision%29))
  (bind _returnvalue (Components|GetOwner))
  (bind _shadowcomponent (Variables|Default|GetShadowComponent))
  (bind _returnvalue_2 (Transformation|GetActorLocation _returnvalue))
  (bind _outhit (Collision|LineTraceByChannel _returnvalue_2 (+ _returnvalue_2 (* (Math|Vector|NegateVector (Transformation|GetActorUpVector _returnvalue)) 1e+03)) "TraceTypeQuery1" false 0 "None"))
  (Transformation|SetWorldLocationAndRotation _shadowcomponent (+ (.Location (Collision|BreakHitResult _outhit)) "0, 0,-3.000000") (Math|Rotator|MakeRotator (.roll (Math|Rotator|MakeRotfromZX (.Normal (Collision|BreakHitResult _outhit)) (Math|Vector|GetForwardVector _shadowcomponent))) (.pitch (Math|Rotator|MakeRotfromZX (.Normal (Collision|BreakHitResult _outhit)) (Math|Vector|GetForwardVector _shadowcomponent))) (.yaw (Transformation|GetActorRotation (Components|GetOwner)))) false false))