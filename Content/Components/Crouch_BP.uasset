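; Crouch_BP is a component that handles crouching for its owning Smol_Character_BP.
; On BeginPlay it casts and caches the owner, then binds its handlers to the character's started and stopped crouching events.
; Each handler sets the character's IsCrouched flag directly and calls Crouch or UnCrouch on it.
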(event Custom|DoCrouch
  (bind _as_smol_character_bp (Variables|Default|GetAs%20Smol%20Character%20BP))
  (Variables|/Game/Smol/Smol_Character_BP.Smol_Character_BP_C|SetIsCrouched? _as_smol_character_bp true)
  (Character|Crouch _as_smol_character_bp))

(event Custom|StopCrouch
  (bind _as_smol_character_bp (Variables|Default|GetAs%20Smol%20Character%20BP))
  (Variables|/Game/Smol/Smol_Character_BP.Smol_Character_BP_C|SetIsCrouched? _as_smol_character_bp false)
  (Character|UnCrouch _as_smol_character_bp))

(event EventBeginPlay
  (bind _assmol_character_bp (Utilities|Casting|CastToSmol_Character_BP (Components|GetOwner)))
  (bind _output_get (Variables|Default|SetAs%20Smol%20Character%20BP _assmol_character_bp))
  (EventDispatchers|BindEventtoStartedCrouching _output_get (delegate Custom|DoCrouch))
  (EventDispatchers|BindEventtoStoppedCrouching _output_get (delegate Custom|StopCrouch)))