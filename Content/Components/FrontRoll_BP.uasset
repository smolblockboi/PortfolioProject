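; FrontRoll is a component that gives its owning Smol character a forward roll attack.
; It binds to the character's AttemptAttack event and, if the character is moving, walking and not already attacking, spawns an attack actor attached to it.
; Tick forces velocity along the forward vector above max walk speed while the roll timer runs.
; The roll flag clears and the attack actor is destroyed when time expires or walking stops.
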(event Custom|StartAttack
  (bind _as_smol_character_bp (Variables|Default|GetAs%20Smol%20Character%20BP))
  (bind _return (CallFunction|CanStartRoll?))
  (if _return
    (bind _returnvalue (Game|SpawnActorfromClass (Variables|Default|GetAttackBP) (Transformation|GetActorTransform _as_smol_character_bp) "Undefined" 0 0))
    (bind _output_get (Variables|Default|SetCurrentAttack _returnvalue))
    (Transformation|AttachActorToActor _output_get (Components|GetOwner) "None" "SnapToTarget" "SnapToTarget" "SnapToTarget" true)
    (Variables|/Game/Smol/Smol_Character_BP.Smol_Character_BP_C|SetIsRollAttacking? _as_smol_character_bp true)
    (Variables|Default|SetRollDuration (/ (Variables|Default|GetBaseRollDuration) 2.0))))

(event EventBeginPlay
  (bind _assmol_character_bp (Utilities|Casting|CastToSmol_Character_BP (Components|GetOwner)))
  (bind _output_get (Variables|Default|SetAs%20Smol%20Character%20BP _assmol_character_bp))
  (EventDispatchers|BindEventtoAttemptAttack _output_get (delegate Custom|StartAttack)))

(event EventTick
  (params (DeltaSeconds :type Float%20%28single-precision%29))
  (bind _as_smol_character_bp (Variables|Default|GetAs%20Smol%20Character%20BP))
  (bind _currentattack (Variables|Default|GetCurrentAttack))
  (bind _charactermovement (Variables|/Script/Engine.Character|GetCharacterMovement _as_smol_character_bp))
  (bind _returnvalue (Pawn|Components|CharacterMovement|IsWalking _charactermovement))
  (if (Math|Boolean|ANDBoolean (> (Variables|Default|GetRollDuration) 0.0) (Variables|/Game/Smol/Smol_Character_BP.Smol_Character_BP_C|GetIsRollAttacking? _as_smol_character_bp) _returnvalue)
    (Variables|Default|SetRollDuration (- (Variables|Default|GetRollDuration) DeltaSeconds))
    (Variables|/Script/Engine.MovementComponent|SetVelocity _charactermovement (* (Transformation|GetActorForwardVector _as_smol_character_bp) (* (Variables|/Script/Engine.CharacterMovementComponent|GetMaxWalkSpeed _charactermovement) 1.5)))
    (elif (or (Variables|/Game/Smol/Smol_Character_BP.Smol_Character_BP_C|GetIsRollAttacking? _as_smol_character_bp) (not _returnvalue))
      (Variables|/Game/Smol/Smol_Character_BP.Smol_Character_BP_C|SetIsRollAttacking? _as_smol_character_bp false)
      (Utilities|IsValid _currentattack
        (:Is%20Valid
          (Actor|DestroyActor _currentattack))))))

(fn CanStartRoll?
  (bind _as_smol_character_bp (Variables|Default|GetAs%20Smol%20Character%20BP))
  (return (Math|Boolean|ANDBoolean (Math|Vector|NotEqual(Vector) (Transformation|GetVelocity _as_smol_character_bp) "0, 0, 0" 0.0001) (Pawn|Components|CharacterMovement|IsWalking (Variables|/Script/Engine.Character|GetCharacterMovement _as_smol_character_bp)) (not (Variables|/Game/Smol/Smol_Character_BP.Smol_Character_BP_C|GetIsRollAttacking? _as_smol_character_bp)) (not (Utilities|IsValid (Variables|Default|GetCurrentAttack))))))