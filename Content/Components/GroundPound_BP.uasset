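; Actor component that gives Smol_Character_BP a ground pound move, triggered by the character's attempt event.
; It runs timed phases: a flying-mode upward hop, a brief hang, then a hard downward impulse with an attached GroundPoundAttack actor spawned.
; The attack's ended events clear character state flags, with a short movement-locked recovery on landing.
; Tick cancels that recovery if the character starts falling.
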(event Custom|DoGroundPound
  (CallFunction|GroundPoundStart)
  (Utilities|FlowControl|Delay 0.3)
  (CallFunction|GroundPoundSpin)
  (Utilities|FlowControl|Delay 0.2)
  (bind _spawnedgroundpound (CallFunction|GroundPoundActivate))
  (EventDispatchers|BindEventtoEndedonGround _spawnedgroundpound (delegate Custom|LandedOnGround))
  (EventDispatchers|BindEventtoEndedEarly _spawnedgroundpound (delegate Custom|EndedEarly)))

(event Custom|EndedEarly
  (bind _as_smol_character_bp (Variables|Default|GetAs%20Smol%20Character%20BP))
  (Variables|/Game/Smol/Smol_Character_BP.Smol_Character_BP_C|SetIsGroundPounding? _as_smol_character_bp false)
  (Variables|/Game/Smol/Smol_Character_BP.Smol_Character_BP_C|SetCharacterCanMove? _as_smol_character_bp true)
  (Variables|/Game/Smol/Smol_Character_BP.Smol_Character_BP_C|SetIsRecoveringFromGroundPound? _as_smol_character_bp false))

(event Custom|LandedOnGround
  (bind _as_smol_character_bp (Variables|Default|GetAs%20Smol%20Character%20BP))
  (Variables|/Game/Smol/Smol_Character_BP.Smol_Character_BP_C|SetIsGroundPounding? _as_smol_character_bp false)
  (Variables|/Game/Smol/Smol_Character_BP.Smol_Character_BP_C|SetIsRecoveringFromGroundPound? _as_smol_character_bp true)
  (Utilities|FlowControl|Delay 0.3)
  (Variables|/Game/Smol/Smol_Character_BP.Smol_Character_BP_C|SetCharacterCanMove? _as_smol_character_bp true)
  (Variables|/Game/Smol/Smol_Character_BP.Smol_Character_BP_C|SetIsRecoveringFromGroundPound? _as_smol_character_bp false))

(event EventBeginPlay
  (bind _assmol_character_bp (Utilities|Casting|CastToSmol_Character_BP (Components|GetOwner)))
  (bind _output_get (Variables|Default|SetAs%20Smol%20Character%20BP _assmol_character_bp))
  (EventDispatchers|BindEventtoAttemptGroundPound _output_get (delegate Custom|DoGroundPound)))

(event EventTick
  (params (DeltaSeconds :type Float%20%28single-precision%29))
  (bind _as_smol_character_bp (Variables|Default|GetAs%20Smol%20Character%20BP))
  (Utilities|IsValid _as_smol_character_bp
    (:Is%20Valid
      (if (and (Variables|/Game/Smol/Smol_Character_BP.Smol_Character_BP_C|GetIsRecoveringFromGroundPound? _as_smol_character_bp) (AI|Components|NavMovement|IsFalling (Variables|/Script/Engine.Character|GetCharacterMovement (Variables|Default|GetAs%20Smol%20Character%20BP))))
        (Variables|/Game/Smol/Smol_Character_BP.Smol_Character_BP_C|SetIsRecoveringFromGroundPound? _as_smol_character_bp false)
        (Variables|/Game/Smol/Smol_Character_BP.Smol_Character_BP_C|SetCharacterCanMove? _as_smol_character_bp true)))))

(fn GroundPoundStart
  (bind _as_smol_character_bp (Variables|Default|GetAs%20Smol%20Character%20BP))
  (bind _returnvalue (Actor|GetComponentbyClass _as_smol_character_bp "/Script/Engine.CharacterMovementComponent"))
  (Variables|/Game/Smol/Smol_Character_BP.Smol_Character_BP_C|SetIsGroundPounding? _as_smol_character_bp true)
  (Variables|/Game/Smol/Smol_Character_BP.Smol_Character_BP_C|SetCharacterCanMove? _as_smol_character_bp false)
  (Pawn|Components|CharacterMovement|SetMovementMode _returnvalue "MOVE_Flying" 0)
  (Components|Movement|StopMovementImmediately _returnvalue)
  (Physics|AddImpulse _returnvalue "0, 0,500.000000" true)
  (return))

(fn GroundPoundActivate
  (bind _as_smol_character_bp (Variables|Default|GetAs%20Smol%20Character%20BP))
  (bind _returnvalue (Actor|GetComponentbyClass _as_smol_character_bp "/Script/Engine.CharacterMovementComponent"))
  (Pawn|Components|CharacterMovement|SetMovementMode _returnvalue "MOVE_Falling" 0)
  (bind _returnvalue_2 (Game|SpawnActorfromClass (Variables|Default|GetGroundPoundAttack) (Transformation|GetActorTransform _as_smol_character_bp) "AlwaysSpawn" 0 0))
  (Transformation|AttachActorToActor _returnvalue_2 (Components|GetOwner) "None" "SnapToTarget" "KeepRelative" "KeepRelative" true)
  (Physics|AddImpulse _returnvalue "0, 0,-10000.000000" true)
  (return _returnvalue_2))

(fn GroundPoundSpin
  (Components|Movement|StopMovementImmediately (Actor|GetComponentbyClass (Variables|Default|GetAs%20Smol%20Character%20BP) "/Script/Engine.CharacterMovementComponent")))