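; BetterSwimming_BP is a swimming helper that detects when it sits at the water surface.
; BelowWaterSphere and AboveWaterSphere set bottom and top in-water flags as they begin or end overlaps with WaterArea_BP actors.
; Each Tick, GetSubmersionState sets IsAtTopOfWater when the bottom sphere is in water and the top one is not.
; The file only tracks this state and applies no movement itself.
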(event OnComponentBeginOverlap(BelowWaterSphere)
  (params (OverlappedComponent :type Primitive%20Component%20Object%20Reference) (OtherActor :type Actor%20Object%20Reference) (OtherComp :type Primitive%20Component%20Object%20Reference) (OtherBodyIndex :type Integer) (bFromSweep :type Boolean) (SweepResult :type Hit%20Result%20Structure%20%28by%20ref%29))
  (Utilities|Casting|CastToWaterArea_BP OtherActor)
  (Variables|Default|SetIsBottomInWater? true))

(event OnComponentEndOverlap(BelowWaterSphere)
  (params (OverlappedComponent :type Primitive%20Component%20Object%20Reference) (OtherActor :type Actor%20Object%20Reference) (OtherComp :type Primitive%20Component%20Object%20Reference) (OtherBodyIndex :type Integer))
  (Utilities|Casting|CastToWaterArea_BP OtherActor)
  (Variables|Default|SetIsBottomInWater? false))

(event OnComponentBeginOverlap(AboveWaterSphere)
  (params (OverlappedComponent :type Primitive%20Component%20Object%20Reference) (OtherActor :type Actor%20Object%20Reference) (OtherComp :type Primitive%20Component%20Object%20Reference) (OtherBodyIndex :type Integer) (bFromSweep :type Boolean) (SweepResult :type Hit%20Result%20Structure%20%28by%20ref%29))
  (Utilities|Casting|CastToWaterArea_BP OtherActor)
  (Variables|Default|SetIsTopInWater? true))

(event OnComponentEndOverlap(AboveWaterSphere)
  (params (OverlappedComponent :type Primitive%20Component%20Object%20Reference) (OtherActor :type Actor%20Object%20Reference) (OtherComp :type Primitive%20Component%20Object%20Reference) (OtherBodyIndex :type Integer))
  (Utilities|Casting|CastToWaterArea_BP OtherActor)
  (Variables|Default|SetIsTopInWater? false))

(event EventTick
  (params (DeltaSeconds :type Float%20%28single-precision%29))
  (CallFunction|GetSubmersionState))

(fn ConstructionScript)

(fn GetSubmersionState
  (Variables|Default|SetIsAtTopOfWater? (and (not (Variables|Default|GetIsTopInWater?)) (Variables|Default|GetIsBottomInWater?))))