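; Actor component that lets Smol_Character_BP grip and hang from ceilings while jump is held, releasing when the button is let go.
; While the character rises in a fall, an upward line trace finds a ceiling, starting the hang and attaching to it.
; Tick then uses Flying mode at reduced speed, snapping height below the surface.
; A floor sphere trace, lost ceiling or physics-simulating surface ends the hang with a jump.
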(event Custom|StopHanging
  (bind _as_smol_character_bp (Variables|Default|GetAs%20Smol%20Character%20BP))
  (bind _charactermovement (Variables|/Script/Engine.Character|GetCharacterMovement _as_smol_character_bp))
  ;[1 1 1] Stop Hanging
  (Variables|Default|SetGripActive false)
  (if (Variables|/Game/Smol/Smol_Character_BP.Smol_Character_BP_C|GetIsHanging? (Variables|Default|GetAs%20Smol%20Character%20BP))
    (Pawn|Components|CharacterMovement|SetMovementMode _charactermovement "MOVE_Falling" 0)
    (Variables|/Game/Smol/Smol_Character_BP.Smol_Character_BP_C|SetIsHanging? (Variables|Default|GetAs%20Smol%20Character%20BP) false)
    (Variables|/Script/Engine.CharacterMovementComponent|SetMaxFlySpeed _charactermovement (Variables|Default|GetDefault%20Fly%20Speed))
    (CallFunction|DetachPlayerfromComponent)))

(event Custom|StartHanging
  (bind _as_smol_character_bp (Variables|Default|GetAs%20Smol%20Character%20BP))
  (bind _charactermovement (Variables|/Script/Engine.Character|GetCharacterMovement _as_smol_character_bp))
  ;[1 1 1] Start Hanging
  (Components|Movement|StopMovementImmediately _charactermovement)
  (Variables|Default|SetDefault%20Fly%20Speed (Variables|/Script/Engine.CharacterMovementComponent|GetMaxFlySpeed _charactermovement))
  (Variables|/Game/Smol/Smol_Character_BP.Smol_Character_BP_C|SetIsHanging? (Variables|Default|GetAs%20Smol%20Character%20BP) true)
  (Variables|/Script/Engine.CharacterMovementComponent|SetMaxFlySpeed _charactermovement 2e+02))

(event Custom|ActivateGrip
  ;[1 1 1] Activate Grip
  (Variables|Default|SetGripActive true))

(event EventBeginPlay
  (bind _assmol_character_bp (Utilities|Casting|CastToSmol_Character_BP (Components|GetOwner)))
  (bind _output_get (Variables|Default|SetAs%20Smol%20Character%20BP _assmol_character_bp))
  (Utilities|FlowControl|Sequence
    (:then_0
      (EventDispatchers|BindEventtoReleasedJump _output_get (delegate Custom|StopHanging)))
    (:then_1
      (EventDispatchers|BindEventtoJumpPressStart _output_get (delegate Custom|ActivateGrip)))))

(event EventTick
  (params (DeltaSeconds :type Float%20%28single-precision%29))
  (bind _as_smol_character_bp (Variables|Default|GetAs%20Smol%20Character%20BP))
  (bind _as_smol_character_bp_2 (Variables|Default|GetAs%20Smol%20Character%20BP))
  (bind _as_smol_character_bp_3 (Variables|Default|GetAs%20Smol%20Character%20BP))
  (bind _returnvalue (Transformation|GetActorLocation _as_smol_character_bp_3))
  (if (Variables|/Game/Smol/Smol_Character_BP.Smol_Character_BP_C|GetIsHanging? (Variables|Default|GetAs%20Smol%20Character%20BP))
    (bind _returnvalue_2 (CallFunction|GetFloorTrace))
    (if _returnvalue_2
      (if (and (Variables|/Game/Smol/Smol_Character_BP.Smol_Character_BP_C|GetIsHanging? _as_smol_character_bp_2) (Variables|Default|GetGripActive)) :!label _label
        (CallFunction|StopHanging :!label _label_2)
        (Character|Jump _as_smol_character_bp_2)
        (Variables|Default|SetGripActive true))
      (else
        (bind (_outhit _washit_) (CallFunction|GetCeilingTrace))
        (if (Math|Boolean|ANDBoolean _washit_ (<= (.z (.Normal (Collision|BreakHitResult _outhit))) 0.0) (Variables|Default|GetGripActive))
          (if (not (Physics|IsSimulatingPhysics (.HitComponent (Collision|BreakHitResult _outhit)) "None"))
            (Pawn|Components|CharacterMovement|SetMovementMode (Variables|/Script/Engine.Character|GetCharacterMovement _as_smol_character_bp_3) "MOVE_Flying" 0)
            (Transformation|SetActorLocation _as_smol_character_bp_3 (Math|Vector|MakeVector (.x _returnvalue) (.y _returnvalue) (- (.Z (Math|Vector|BreakVector (.Location (Collision|BreakHitResult _outhit)))) (Variables|Default|GetGripOffset))) true false)
            (else
              (goto _label_2)))
          (else
            (goto _label)))))
    (elif (and (>= (.z (Transformation|GetVelocity _as_smol_character_bp)) 0.0) (AI|Components|NavMovement|IsFalling (Variables|/Script/Engine.Character|GetCharacterMovement _as_smol_character_bp)))
      (bind (_outhit_2 _washit__2) (CallFunction|GetCeilingTrace))
      (if (Math|Boolean|ANDBoolean _washit__2 (Variables|Default|GetGripActive) (< (.z (.Normal (Collision|BreakHitResult _outhit_2))) 0.0))
        (CallFunction|StartHanging)
        (CallFunction|AttachPlayertoComponent (.HitComponent (Collision|BreakHitResult _outhit_2)))))))

(fn GetCeilingTrace
  (bind _as_smol_character_bp (Variables|Default|GetAs%20Smol%20Character%20BP))
  (bind _returnvalue (Transformation|GetActorLocation _as_smol_character_bp))
  (bind (_outhit _returnvalue_2) (Collision|LineTraceByChannel _returnvalue (- _returnvalue (* (Math|Vector|NegateVector (Math|Vector|GetUpVector (Transformation|GetActorRotation _as_smol_character_bp))) (Variables|Default|GetCeilingDistance))) "TraceTypeQuery1" false 0 (Variables|Default|GetDraw%20Debug%20Type)))
  (return _outhit _returnvalue_2))

(fn GetFloorTrace
  (bind _as_smol_character_bp (Variables|Default|GetAs%20Smol%20Character%20BP))
  (bind _returnvalue (Transformation|GetActorLocation _as_smol_character_bp))
  (bind (_outhit _returnvalue_2) (Collision|SphereTraceByChannel _returnvalue (+ _returnvalue (* (Math|Vector|NegateVector (Math|Vector|GetUpVector (Transformation|GetActorRotation _as_smol_character_bp))) (Variables|Default|GetFloorDistance))) (Variables|Default|GetFloorSphereTraceRadius) "TraceTypeQuery1" false 0 (Variables|Default|GetDraw%20Debug%20Type)))
  (return _outhit _returnvalue_2))