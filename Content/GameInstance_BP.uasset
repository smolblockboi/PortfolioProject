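; Game instance that holds the player's progress: unlocked abilities, coin and red coin counts, and respawn location.
; Abilities are stored as component classes; each new unlock re-adds the whole list to the player character without checking for existing components.
; Respawn spawns a new character if destroyed, otherwise teleports the current one.
; Both respawn paths reapply abilities, then set the player reference from the spawn result.
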(event Custom|CoinCollected
  (bind _result (Math|Integer|IncrementInt (Variables|Default|GetCoinsCollected))
    (:%20%20
      (Variables|Default|SetCoinsCollected _result))))

(event Custom|SetPlayerRespawnLocation
  (params (NewLocation :type Vector))
  (Variables|Default|SetPlayerRespawnLocation NewLocation))

(event Custom|UnlockAbility
  (params (NewAbility :type Actor%20Component%20Class%20Reference))
  (bind _unlockedabilities (Variables|Default|GetUnlockedAbilities))
  (if (== (Utilities|Array|FindItem _unlockedabilities NewAbility) -1)
    (Utilities|Array|Add _unlockedabilities NewAbility)
    (Development|PrintString (Utilities|String|Append "Unlocked " (Utilities|GetClassDisplayName NewAbility)))
    (CallFunction|AssignUnlockedAbilities)))

(event Custom|AssignUnlockedAbilities
  (bind _assmol_character_bp (Utilities|Casting|CastToSmol_Character_BP (Game|Player|GetPlayerPawn 0)))
  (for _array_element (Variables|Default|GetUnlockedAbilities)
    (Game|AddComponentbyClass _assmol_character_bp _array_element)
    (Development|PrintString (Utilities|String|Append "Equipped " (Utilities|GetClassDisplayName _array_element)))))

(event Custom|RedCoinCollected
  (bind _result (Math|Integer|IncrementInt (Variables|Default|GetRedCoinsCollected))
    (:%20%20
      (Variables|Default|SetRedCoinsCollected _result))))

(event Custom|RespawnPlayer
  (params (WasDestroyed? :type Boolean))
  (bind _playerrespawnlocation (Variables|Default|GetPlayerRespawnLocation))
  (bind _returnvalue (Math|Transform|MakeTransform _playerrespawnlocation))
  (if WasDestroyed?
    (bind _returnvalue_2 (Game|SpawnActorfromClass "/Game/Smol/Smol_Character_BP.Smol_Character_BP_C" _returnvalue "Undefined" 0 0))
    (else
      (Transformation|SetActorTransform (Variables|Default|GetSmolPlayerRef) _returnvalue false true)))
  (CallFunction|AssignUnlockedAbilities)
  (Variables|Default|SetSmolPlayerRef _returnvalue_2))